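; BP_HealthComponent is a health component that tracks an actor's current health and signals when it dies.
; It fills CurrentHealth from MaxHealth on BeginPlay, and TakeDamage subtracts the damage amount without clamping.
; When the depletion check finds health at or below zero, Die calls the OnDeath dispatcher.
; The owner is not destroyed here, as the DestroyActor node is left unconnected.
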(event `self.ReceiveBeginPlay`
  (set `self.CurrentHealth` (`self.MaxHealth`)))

(event `TakeDamage`
  (params (DamageAmount :type "Float (double-precision)"))
  (set `self.CurrentHealth` (- (`self.CurrentHealth`) DamageAmount))
  (if (`self.IsHealthIsDepleted`)
    (`self.Die`)))

(event `Die`
  (`self.OnDeath`))

(fn `IsHealthIsDepleted`
  (returns (ReturnValue :type Boolean))
  (return (<= (`self.CurrentHealth`) 0.0)))