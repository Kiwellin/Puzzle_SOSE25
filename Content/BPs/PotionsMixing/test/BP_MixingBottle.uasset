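; BP_MixingBottle is an interactable bottle that mixes its current color with a held color potion in a potion-mixing system.
; Interact casts the pickup to BP_ColorPotion, then CheckColor searches the Recipes data table for a row pairing both colors in either order.
; A match stores the recipe's result color and prints it.
; Otherwise LiquidGoPOOF prints a message and sets the bottle to a fixed enum color.
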(event `Liquid Go POOF`
  (`KismetSystemLibrary.PrintString` "Color go POOF")
  (set `self.ColorInMixingBottle` "NewEnumerator3"))

(fn `CheckColor`
  (params (PotionInHand :type "/Game/BPs/PotionsMixing/test/BP_ColorPotion Object Reference"))
  (bind _colorinmixingbottle (`self.ColorInMixingBottle`))
  (bind _bottleinhandcolor (`self.BottleInHandColor`))
  (bind (_colorname _color1) (break `/Game/BPs/PotionsMixing/test/S_ColorRecipe` (`self.Out Row`)))
  (bind (_colorname_2 _color1_2 _color2) (break `/Game/BPs/PotionsMixing/test/S_ColorRecipe` (`self.Out Row`)))
  (bind _returnvalue (`|EnumEquality` _color1 _bottleinhandcolor))
  (set `self.BottleInHandColor` (`/Game/BPs/PotionsMixing/test/BP_ColorPotion.Color` PotionInHand))
  (bind _outrownames (`DataTableFunctionLibrary.GetDataTableRowNames` (`self.Recipes`)))
  (for _array_element _outrownames
    (bind _returnvalue_2 (`|GetDataTableRow` (`self.Recipes`) _array_element)
      (:`then`
        (set `self.Out Row` _returnvalue_2)
        (if (or (`|EnumEquality` _color1 _colorinmixingbottle) _returnvalue)
          (if (`|EnumEquality` (`.Color2_8_3815C9C44E5A611DCDADBB8ABE94CDB1` (break `/Game/BPs/PotionsMixing/test/S_ColorRecipe` (`self.Out Row`))) (select `bool` _returnvalue :`false` _bottleinhandcolor :`true` _colorinmixingbottle))
            (`KismetSystemLibrary.PrintString` (`|GetEnumeratorNameAsString` _color1_2))
            (`KismetSystemLibrary.PrintString` (`|GetEnumeratorNameAsString` _color2))
            (set `self.NewColorInMixingBottle` _colorname_2)
            (set `self.ColorInMixingBottle` (`self.NewColorInMixingBottle`))
            (set `self.FoundColorMatch` true)
            (return)
            (else
              _)))
        (set `self.FoundColorMatch` false))))
  (return))

(fn `Interact`
  (params (`Player Character` :type "/Game/BPs/BP_FirstPersonCharacter Object Reference") (PickUpItem :type "/Game/BPs/BP_PickUpItem Object Reference"))
  (returns (UsedUpPickUp :type Boolean) (MultiUseItemused :type Boolean))
  (`/Engine/EditorBlueprintResources/StandardMacros.IsValid` PickUpItem
    (:`Is Valid`
      (bind _asbp_color_potion (cast `/Game/BPs/PotionsMixing/test/BP_ColorPotion` PickUpItem)
        (:`then`
          (`self.CheckColor` _asbp_color_potion)
          (`self.PrintColor`)
          (return false true))
        (:`CastFailed`
          (return false false))))))

(fn `PrintColor`
  (if (`self.FoundColorMatch`)
    (`KismetSystemLibrary.PrintString` (`|GetEnumeratorNameAsString` (`self.ColorInMixingBottle`)))
    (else
      (`self.Liquid Go POOF`))))

(fn `UserConstructionScript`
  (`parent.UserConstructionScript`))