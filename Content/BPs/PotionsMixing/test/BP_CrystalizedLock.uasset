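; Crystal lock actor in the potion-mixing puzzle that steps through an array of colors and destroys itself after the last is solved.
; Interacting with a mixing bottle runs CheckColor, which tests the bottle's color against the current lock color using rows of the Contrasts data table.
; A match advances the lock, while a failed check calls LiquidGoPOOF on the bottle.
; Feedback is currently only debug prints.
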(event `self.ReceiveBeginPlay`
  (bind _output_get (set `self.LockColor` (`|GetArrayItem` (`self.ColorArray`))))
  (`KismetSystemLibrary.PrintString` (`|GetEnumeratorNameAsString` _output_get)))

(event `NextColor`
  (bind _output_get (set `self.ColorArrayIndex` (+ 1 (`self.ColorArrayIndex`))))
  (`KismetSystemLibrary.PrintString` (`KismetStringLibrary.Conv_IntToString` _output_get))
  (if (== (`self.ColorArrayIndex`) (`KismetArrayLibrary.Array_Length` (`self.ColorArray`)))
    (`self.DestroyCrystal`)
    (else
      (bind _output_get_2 (set `self.LockColor` (`|GetArrayItem` (`self.ColorArray`) (`self.ColorArrayIndex`))))
      (`KismetSystemLibrary.PrintString` (`|GetEnumeratorNameAsString` _output_get_2)))))

(event `DestroyCrystal`
  (`KismetSystemLibrary.PrintString` "crystalGoPOOD")
  (`KismetSystemLibrary.Delay` 0.5)
  (`self.K2_DestroyActor`))

(fn `CheckColor`
  (params (MixingBottle :type "/Game/BPs/PotionsMixing/test/BP_MixingBottle Object Reference"))
  (returns (FoundColorMatch :type Boolean))
  (bind _bottleinhandcolor (`self.BottleInHandColor`))
  (bind _lockcolor (`self.LockColor`))
  (bind (_lockcolor_2 _potioncontrast) (break `/Game/BPs/PotionsMixing/test/S_CrystalLockContrast` (`self.Out Row`)))
  (bind (_lockcolor_3 _potioncontrast_2) (break `/Game/BPs/PotionsMixing/test/S_CrystalLockContrast` (`self.Out Row`)))
  (bind _returnvalue (`|EnumEquality` _potioncontrast_2 _bottleinhandcolor))
  (set `self.BottleInHandColor` (`/Game/BPs/PotionsMixing/test/BP_MixingBottle.ColorInMixingBottle` MixingBottle))
  (if (`|EnumInequality` (`self.BottleInHandColor`) "NewEnumerator3")
    (bind _outrownames (`DataTableFunctionLibrary.GetDataTableRowNames` (`self.Contrasts`)))
    (for _array_element _outrownames
      (bind _returnvalue_2 (`|GetDataTableRow` (`self.Contrasts`) _array_element)
        (:`then`
          (set `self.Out Row` _returnvalue_2)
          (if (or (`|EnumEquality` _lockcolor_3 _lockcolor) _returnvalue)
            (if (`|EnumEquality` (`.LockColor_10_127BD7F347C73B46EEEF3C844CC465E3` (break `/Game/BPs/PotionsMixing/test/S_CrystalLockContrast` (`self.Out Row`))) (select `bool` _returnvalue :`false` _bottleinhandcolor :`true` _lockcolor))
              (`KismetSystemLibrary.PrintString` (`|GetEnumeratorNameAsString` _lockcolor_2))
              (`KismetSystemLibrary.PrintString` (`|GetEnumeratorNameAsString` _potioncontrast))
              (bind _output_get (set `self.FoundColorMatch` true))
              (return _output_get)
              (else
                _)))
          (set `self.FoundColorMatch` false))))
    (return (`self.FoundColorMatch`))
    (else
      (`KismetSystemLibrary.PrintString` "Should Fill the bottle before attempting to solve lock"))))

(fn `Interact`
  (params (`Player Character` :type "/Game/BPs/BP_FirstPersonCharacter Object Reference") (PickUpItem :type "/Game/BPs/BP_PickUpItem Object Reference"))
  (returns (UsedUpPickUp :type Boolean) (MultiUseItemused :type Boolean))
  (`/Engine/EditorBlueprintResources/StandardMacros.IsValid` PickUpItem
    (:`Is Valid`
      (bind _asbp_mixing_bottle (cast `/Game/BPs/PotionsMixing/test/BP_MixingBottle` PickUpItem)
        (:`then`
          (bind _foundcolormatch (`self.CheckColor` _asbp_mixing_bottle))
          (`self.PrintColor` _asbp_mixing_bottle _foundcolormatch)
          (return false true))
        (:`CastFailed`
          (return false false))))))

(fn `PrintColor`
  (params (`Mixing Bottle` :type "/Game/BPs/PotionsMixing/test/BP_MixingBottle Object Reference") (FoundColorMatch :type Boolean))
  (if FoundColorMatch
    (`KismetSystemLibrary.PrintString` "correct")
    (`self.NextColor`)
    (else
      (`KismetSystemLibrary.PrintString` "Color go POOF")
      (`/Game/BPs/PotionsMixing/test/BP_MixingBottle.Liquid Go POOF` `Mixing Bottle`))))

(fn `UserConstructionScript`)