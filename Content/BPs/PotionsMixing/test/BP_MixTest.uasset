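; BP_MixTest is a test Blueprint for potion color mixing, checking two bottle colors against a recipe table.
; On Interact it loops through every Recipes row, comparing Color1 and Color2 each to either the mixing-bottle or in-hand color, so order is ignored.
; Each row prints its resulting ColorName on a match or "false" otherwise, without stopping at the first match or producing a potion.
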(event `/Game/BPs/interfaces/InteractionInterface.Interact`
  (params (`Player Character` :type "/Game/BPs/BP_FirstPersonCharacter Object Reference"))
  (bind (_colorname _color1) (break `/Game/BPs/PotionsMixing/test/S_ColorRecipe` (`self.Out Row`)))
  (bind (_colorname_2 _color1_2 _color2) (break `/Game/BPs/PotionsMixing/test/S_ColorRecipe` (`self.Out Row`)))
  (bind _outrownames (`DataTableFunctionLibrary.GetDataTableRowNames` (`self.Recipes`)))
  (for _array_element _outrownames
    (bind _returnvalue (`|GetDataTableRow` (`self.Recipes`) _array_element)
      (:`then`
        (set `self.Out Row` _returnvalue)
        (if (or (`|EnumEquality` _color1 (`self.ColorInMixingBottle`)) (`|EnumEquality` _color1 (`self.BottleInHandColor`)))
          (if (or (`|EnumEquality` _color2 (`self.ColorInMixingBottle`)) (`|EnumEquality` _color2 (`self.BottleInHandColor`)))
            (`KismetSystemLibrary.PrintString` (`.ColorName_2_127BD7F347C73B46EEEF3C844CC465E3` (break `/Game/BPs/PotionsMixing/test/S_ColorRecipe` (`self.Out Row`))))
            (else
              (`KismetSystemLibrary.PrintString` "false" :!label _label)))
          (else
            (goto _label)))))))

(fn `UserConstructionScript`
  (`parent.UserConstructionScript`))