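; Statue rotation puzzle actor, named for a secret compartment, that tracks which statues are correct.
; CheckIfAllCorrect adds each reported statue to CorrectStatues and prints a debug message when exactly three are stored.
; Nothing removes entries, the NewParam input is unused, and no compartment opening is implemented.
; The Interact override only calls the parent and returns false.
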(event `CheckIfAllCorrect`
  (params (NewParam :type Boolean) (CorrectStatue :type "/Game/BPs/Statues/BP_StatuesRotate Object Reference"))
  (`KismetArrayLibrary.Array_Add` (`self.CorrectStatues`) CorrectStatue)
  (if (== (`KismetArrayLibrary.Array_Length` (`self.CorrectStatues`)) 3)
    (`KismetSystemLibrary.PrintString` "all 3 correct")))

(fn `Interact`
  (params (`Player Character` :type "/Game/BPs/BP_FirstPersonCharacter Object Reference") (PickUpActor :type "/Game/BPs/Pickups/BP_PickUpActor Object Reference"))
  (returns (UsedUpPickUp :type Boolean))
  (`parent.Interact` `Player Character` null)
  (return false))

(fn `UserConstructionScript`
  (`parent.UserConstructionScript`))