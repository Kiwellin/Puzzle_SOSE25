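; A rotating puzzle statue that the player turns in 45-degree steps until it reaches its correct rotation, optionally gated behind placing a required item.
; Interacting attaches a matching item to ItemPivot to clear that gate; later interactions turn it in a direction chosen by which side of the player's view it sits on.
; Tick smoothly lerps the cylinder toward the target; a correct statue stops turning and asks MainStatue to check whether all are correct.
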(event `Interact_1_1`
  (params (`Player Character` :type "/Game/BPs/BP_FirstPersonCharacter Object Reference") (PickUpActor :type "/Game/BPs/Pickups/BP_PickUpActor Object Reference"))
  (bind _item (`/Game/BPs/BP_FirstPersonCharacter.Item` `Player Character`))
  (`self.Interacted`)
  (`/Engine/EditorBlueprintResources/StandardMacros.IsValid` _item
    (:`Is Valid`
      (if (== _item (`self.CorrectItem`))
        (set `self.NeedsItem` false)
        (`/Game/BPs/BP_PickUpItem.ChangeParents` _item (`self.ItemPivot`))
        (`/Game/BPs/BP_FirstPersonCharacter.Remove Item` `Player Character`)))))

(event `self.ReceiveTick`
  (params (DeltaSeconds :type "Float (single-precision)"))
  (`SceneComponent.K2_SetRelativeRotation` (`self.Cylinder`) (`KismetMathLibrary.RLerp` (`SceneComponent.RelativeRotation` (`self.Cylinder`)) (`KismetMathLibrary.MakeRotator` 0.0 0.0 (`self.TargetRotation`)) (* (`GameplayStatics.GetWorldDeltaSeconds`) 15.0) true) false false))

(event `Interacted`
  (if (not (`self.NeedsItem`))
    (bind _is_correct (`self.CheckIfCorrect`))
    (if (not _is_correct)
      (`self.Get RotationDirection`)
      (`self.SetTargetRotation`)
      (`KismetSystemLibrary.Delay` 0.2)
      (bind _is_correct_2 (`self.CheckIfCorrect`))
      (bind _output_get (set `self.Is Correct` _is_correct_2))
      (if _output_get
        (`/Game/BPs/Statues/BP_StatuesRotateSecretCompartment.CheckIfAllCorrect` (`self.MainStatue`) false self)))))

(fn `CheckIfCorrect`
  (returns (`Is Correct` :type Boolean))
  (if (== (`self.TargetRotation`) (`self.CorrectRotation`))
    (`KismetSystemLibrary.PrintString` "YIPIEEEEEEE")
    (return true)
    (else
      (return false))))

(fn `Get RotationDirection`
  (bind (_location _rotation) (`Controller.GetPlayerViewPoint` (`GameplayStatics.GetPlayerController` 0)))
  (if (> (`KismetMathLibrary.Dot_VectorVector` (`KismetMathLibrary.Vector_Normal2D` (- (`self.K2_GetActorLocation`) _location)) (`KismetMathLibrary.Vector_Normal2D` (`KismetMathLibrary.GetRightVector` _rotation))) 0.0)
    (set `self.RotDirection` 1.0)
    (else
      (set `self.RotDirection` -1.0)))
  (return))

(fn `Interact`
  (params (`Player Character` :type "/Game/BPs/BP_FirstPersonCharacter Object Reference") (PickUpItem :type "/Game/BPs/BP_PickUpItem Object Reference"))
  (returns (UsedUpPickUp :type Boolean))
  (`self.Interacted`)
  (`/Engine/EditorBlueprintResources/StandardMacros.IsValid` PickUpItem
    (:`Is Valid`
      (if (== PickUpItem (`self.CorrectItem`))
        (set `self.NeedsItem` false)
        (`/Game/BPs/BP_PickUpItem.ChangeParents` PickUpItem (`self.ItemPivot`))
        (return true)))))

(fn `SetTargetRotation`
  (bind _returnvalue (+ (`self.TargetRotation`) (* 45.0 (`self.RotDirection`))))
  (`|ExecutionSequence`
    (:`then_0`
      (if (> _returnvalue 360.0)
        (set `self.TargetRotation` 0.0)))
    (:`then_1`
      (if (< _returnvalue 0.0)
        (set `self.TargetRotation` 360.0)))
    (:`then_2`
      (set `self.TargetRotation` _returnvalue))))

(fn `UserConstructionScript`
  (`parent.UserConstructionScript`))