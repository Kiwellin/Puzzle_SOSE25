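; Possessable bell puzzle where the player cycles through four highlighted bells and strikes them to enter a code.
; If a bell is missing, interacting with the correct pickup consumes it, reveals the hidden bell and enables possession.
; Each strike plays a timeline wobble that locks selection and appends the bell's sound ID, capped by the sound-code DataTable's column count.
; A match with the target code currently only prints a message.
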(event `self.ReceiveBeginPlay`
  (`parent.ReceiveBeginPlay`)
  (set `self.Bells` (`|MakeArray` (`self.Bell1`) (`self.Bell2`) (`self.Bell3`) (`self.Bell4`)))
  (bind _outrownames (`DataTableFunctionLibrary.GetDataTableRowNames` (`self.DT Sound Codes`)))
  (bind _output_get (set `self.Out Row Names` _outrownames)))

(event `EnhancedInput|/Game/Input/Actions/IA_ExitPuzzle`
  (params (ActionValue :type Boolean) (ElapsedSeconds :type "Float (double-precision)") (TriggeredSeconds :type "Float (double-precision)") (InputAction :type "InputAction Object Reference" :default "/Game/Input/Actions/IA_ExitPuzzle.IA_ExitPuzzle"))
  (:`Triggered`
    (`self.Return to Character`)))

(event `EnhancedInput|/Game/Input/Actions/IA_NavigateRight`
  (params (ActionValue :type Boolean) (ElapsedSeconds :type "Float (double-precision)") (TriggeredSeconds :type "Float (double-precision)") (InputAction :type "InputAction Object Reference" :default "/Game/Input/Actions/IA_NavigateRight.IA_NavigateRight"))
  (:`Triggered`
    (if (`self.CanSelectNext`)
      (`self.Navigate Bells` 1))))

(event `self.Return to Character`
  (`parent.Return to Character`)
  (`self.UpdateHighlightOfSelectedBell` false))

(event `EnhancedInput|/Game/Input/Actions/IA_NavigateLeft`
  (params (ActionValue :type Boolean) (ElapsedSeconds :type "Float (double-precision)") (TriggeredSeconds :type "Float (double-precision)") (InputAction :type "InputAction Object Reference" :default "/Game/Input/Actions/IA_NavigateLeft.IA_NavigateLeft"))
  (:`Triggered`
    (if (`self.CanSelectNext`)
      (`self.Navigate Bells` -1))))

(event `EnhancedInput|/Game/Input/Actions/IA_Interact`
  (params (ActionValue :type Boolean) (ElapsedSeconds :type "Float (double-precision)") (TriggeredSeconds :type "Float (double-precision)") (InputAction :type "InputAction Object Reference" :default "/Game/Input/Actions/IA_Interact.IA_Interact"))
  (:`Triggered`
    (if (`self.CanSelectNext`)
      (`TimelineComponent.SetPlayRate` (`self.Movebell`) 5.0)
      (`TimelineComponent.PlayFromStart` (`self.Movebell`))
      (`self.AddToCode`)
      (`self.CheckCode`))))

(fn `AddToCode`
  (bind _currentcode (`self.CurrentCode`))
  ; Get Code  length
  (bind _outcolumnnames (`DataTableFunctionLibrary.GetDataTableColumnNames` (`self.DT Sound Codes`)))
  (if (< (`KismetArrayLibrary.Array_Length` _currentcode) (`KismetArrayLibrary.Array_Length` _outcolumnnames))
    (`KismetArrayLibrary.Array_Add` _currentcode (`/Game/BPs/BellPuzzle/BP_SMBell.SoundInt` (`self.GetSelectedBell`)))))

(fn `CheckCode`
  (if (`KismetArrayLibrary.Array_Identical` (`self.Code`) (`self.CurrentCode`))
    (`KismetSystemLibrary.PrintString` "is correct")))

(fn `CheckForBell`
  (params (PickUpItem :type "/Game/BPs/BP_PickUpItem Object Reference"))
  (returns (UsedPickup :type Boolean))
  (`/Engine/EditorBlueprintResources/StandardMacros.IsValid` PickUpItem
    (:`Is Valid`
      (if (== PickUpItem (`self.CorrectItem`))
        (set `self.CanBePossessed` true)
        (`/Game/BPs/BP_PickUpItem.DestroySelf` PickUpItem)
        (`self.UnhideLastBell`)
        (set `self.NeedsItem` false)
        (return true)
        (else
          (return false))))))

(fn `GetSelectedBell`
  (returns (Output :type "/Game/BPs/BellPuzzle/BP_SMBell Object Reference"))
  (return (`|GetArrayItem` (`self.Bells`) (`self.CurrentPieceIndex`))))

(fn `Interact`
  (params (`Player Character` :type "/Game/BPs/BP_FirstPersonCharacter Object Reference") (PickUpItem :type "/Game/BPs/BP_PickUpItem Object Reference"))
  (returns (UsedUpPickUp :type Boolean) (MultiUseItemused :type Boolean))
  (`parent.Interact` `Player Character` PickUpItem)
  (if (`self.NeedsItem`)
    (bind _usedpickup (`self.CheckForBell` PickUpItem))
    (return _usedpickup false)
    (else
      (`self.UpdateHighlightOfSelectedBell` true)
      (return false false))))

(fn `Navigate Bells`
  (params (Direction :type Integer))
  (`self.UpdateHighlightOfSelectedBell` false)
  (set `self.CurrentPieceIndex` (+ (`self.CurrentPieceIndex`) Direction))
  (`|ExecutionSequence`
    (:`then_0`
      ;[1 1 1] Make sure index not too high
      (if (> (`self.CurrentPieceIndex`) (`KismetArrayLibrary.Array_LastIndex` (`self.Bells`)))
        (set `self.CurrentPieceIndex` (- (`self.CurrentPieceIndex`) (`KismetArrayLibrary.Array_Length` (`self.Bells`))))))
    (:`then_1`
      ;[1 1 1] Make sure index not too low
      (if (< (`self.CurrentPieceIndex`) 0)
        (set `self.CurrentPieceIndex` (+ (`self.CurrentPieceIndex`) (`KismetArrayLibrary.Array_Length` (`self.Bells`))))))
    (:`then_2`
      ;[1 1 1] Update highlight
      (`self.UpdateHighlightOfSelectedBell` true))))

(fn `UnhideLastBell`
  (`SceneComponent.SetVisibility` (`self.Bell3`) true false))

(fn `UpdateHighlightOfSelectedBell`
  (params (bEnabled :type Boolean))
  (`MeshComponent.SetOverlayMaterial` (`self.GetSelectedBell`) (select `bool` bEnabled :`true` "/Game/Materials/MI_ButtonHighlight.MI_ButtonHighlight" :!type "MaterialInterface Object Reference")))

(fn `UserConstructionScript`
  (`parent.UserConstructionScript`))