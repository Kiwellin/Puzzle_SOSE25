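; Well puzzle actor that winds a bucket up when its parent class's ItemIsCorrect event fires.
; The event runs the parent logic, then Rotate records the bucket actor's current Z and plays a timeline.
; The timeline spins the cylinder three full turns in yaw while lerping the bucket's Z to BucketDistancUp, an absolute target rather than an offset.
; The bucket's world location feeds a relative-location setter.
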(event `self.ItemIsCorrect`
  (`parent.ItemIsCorrect`)
  (`self.Rotate`))

(event `Rotate`
  (bind _bucket (`self.Bucket`))
  (bind (_returnvalue_x _returnvalue_y) (`KismetMathLibrary.BreakVector` (`self.K2_GetActorLocation` _bucket)))
  (bind (_returnvalue_x_2 _returnvalue_y_2 _returnvalue_z) (`KismetMathLibrary.BreakVector` (`self.K2_GetActorLocation` (`self.Bucket`))))
  (set `self.BucketStartLoc` _returnvalue_z)
  (bind (_direction _newtrack_1) (`Timeline|Timeline`)
    (:`Update`
      (`SceneComponent.K2_SetRelativeRotation` (`self.Cylinder`) (`KismetMathLibrary.MakeRotator` 0.0 0.0 (`KismetMathLibrary.Lerp` 0.0 1080.0 _newtrack_1)) false false)
      (`self.K2_SetActorRelativeLocation` _bucket (`KismetMathLibrary.MakeVector` _returnvalue_x _returnvalue_y (`KismetMathLibrary.Lerp` (`self.BucketStartLoc`) (`self.Bucket Distanc Up`) _newtrack_1)) false false))))

(fn `UserConstructionScript`
  (`parent.UserConstructionScript`))