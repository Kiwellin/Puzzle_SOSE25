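; Sorting puzzle chest whose lid opens further as its stone placement targets report correct.
; On BeginPlay it binds OpenMore to the CheckIfAllCorrect dispatcher of four PlaceItemTarget references.
; Each call increments CorrectStones and raises LidOpenFull to that count's fraction of four, negated, so the angle grows exponentially rather than linearly.
; A timeline lerps the Pivot's roll from the previous angle to the new one, which is also printed for debugging.
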(event `self.ReceiveBeginPlay`
  (add `/Game/BPs/InventoryAndPlacePuzzle/BP_PlaceItemTarget.CheckIfAllCorrect` (`self.PlaceItemTarget_01`) (delegate `OpenMore`))
  (add `/Game/BPs/InventoryAndPlacePuzzle/BP_PlaceItemTarget.CheckIfAllCorrect` (`self.PlaceItemTarget_02`) (delegate `OpenMore`))
  (add `/Game/BPs/InventoryAndPlacePuzzle/BP_PlaceItemTarget.CheckIfAllCorrect` (`self.PlaceItemTarget_04`) (delegate `OpenMore`))
  (add `/Game/BPs/InventoryAndPlacePuzzle/BP_PlaceItemTarget.CheckIfAllCorrect` (`self.PlaceItemTarget_03`) (delegate `OpenMore`)))

(event `OpenMore`
  (bind _returnvalue (* (`KismetMathLibrary.MultiplyMultiply_FloatFloat` (`self.LidOpenFull`) (`self.AddMoreOpen`)) -1.0))
  (set `self.CorrectStones` (+ (`self.CorrectStones`) 1))
  (set `self.AddMoreOpen` (/ (`KismetMathLibrary.Conv_IntToDouble` (`self.CorrectStones`)) 4.0))
  (set `self.OpenAmount` _returnvalue)
  (`KismetSystemLibrary.PrintString` (`KismetStringLibrary.Conv_DoubleToString` _returnvalue))
  (bind (_direction _newtrack_0) (`Timeline|OpenChestMore` :!via `PlayFromStart`)
    (:`Update`
      (`SceneComponent.K2_SetRelativeRotation` (`self.pivot`) (`KismetMathLibrary.MakeRotator` (`KismetMathLibrary.Lerp` (`self.OldAmount`) (`self.OpenAmount`) _newtrack_0)) false false))
    (:`Finished`
      (set `self.OldAmount` (`self.OpenAmount`)))))

(fn `UserConstructionScript`)