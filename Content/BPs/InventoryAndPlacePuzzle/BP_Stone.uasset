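; BP_Stone is an interactable stone actor for the sorting puzzle in the inventory-and-place puzzle system.
; Its Interact function casts the stone's attach parent to BP_SortingPuzzlePlace.
; If that place's ItemCorrect flag is true, it calls RemoveStone on the place and returns false.
; The event graph holds only disabled default events, so all of the stone's own logic lives in Interact.
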(fn `Interact`
  (params (`Player Character` :type "/Game/BPs/BP_FirstPersonCharacter Object Reference") (PickUpItem :type "/Game/BPs/BP_PickUpItem Object Reference"))
  (returns (UsedUpPickUp :type Boolean))
  (bind _asbp_sorting_puzzle_place (cast `/Game/BPs/InventoryAndPlacePuzzle/BP_SortingPuzzlePlace` (`self.GetAttachParentActor`)))
  (if (`/Game/BPs/InventoryAndPlacePuzzle/BP_PlaceItemTarget.ItemCorrect` _asbp_sorting_puzzle_place)
    (`/Game/BPs/InventoryAndPlacePuzzle/BP_SortingPuzzlePlace.RemoveStone` _asbp_sorting_puzzle_place)
    (return false)))

(fn `UserConstructionScript`
  (`parent.UserConstructionScript`))