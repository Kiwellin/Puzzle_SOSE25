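; BP_PlaceItemTarget is an interactable puzzle slot that accepts a held pickup and checks whether it is the correct item.
; Interact reparents the item to PlaceBowlHere, enables its collision and reports the pickup as used.
; A match with CorrectItem fires the CheckIfAllCorrect and ItemPlacedCorrect dispatchers, sets ItemCorrect and disables item collision unless re-pickup is allowed.
; An offering-bowl ingredient check exists but is disconnected from the live flow.
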(event `CheckPlacedItem`
  (if (== (`self.PlacedItem`) (`self.CorrectItem`))
    (`self.ItemIsCorrect`)
    (set `self.ItemCorrect` true)))

(event `ItemIsCorrect`
  (`self.CheckIfAllCorrect`)
  (`self.ItemPlacedCorrect`)
  (if (not (`self.CanPickUpItemAgain`))
    (`self.SetActorEnableCollision` (`self.PlacedItem`) false)))

(fn `CheckIfItemIsOfferingBowl`
  (returns (ReturnValue :type Boolean))
  (bind _asbp_offering_bowl (cast `/Game/BPs/Sacrifice/BP_OfferingBowl` (`self.PlacedItem`))
    (:`then`
      (bind _addedingredient (`/Game/BPs/Sacrifice/BP_OfferingBowl.AddedIngredient` _asbp_offering_bowl))
      (`/Engine/EditorBlueprintResources/StandardMacros.IsValid` _addedingredient
        (:`Is Valid`
          (if (== (`GameplayStatics.GetObjectClass` _addedingredient) (`self.CorrectIngredient`))
            (return true)))
        (:`Is Not Valid`
          (return false))))
    (:`CastFailed`
      (return true))))

(fn `Interact`
  (params (`Player Character` :type "/Game/BPs/BP_FirstPersonCharacter Object Reference") (PickUpItem :type "/Game/BPs/BP_PickUpItem Object Reference"))
  (returns (UsedUpPickUp :type Boolean) (MultiUseItemused :type Boolean))
  (`/Engine/EditorBlueprintResources/StandardMacros.IsValid` PickUpItem
    (:`Is Valid`
      (`KismetSystemLibrary.PrintString` "Hello")
      (set `self.PlacedItem` PickUpItem)
      (`/Game/BPs/BP_PickUpItem.ChangeParents` PickUpItem (`self.PlaceBowlHere`))
      (`PrimitiveComponent.SetCollisionEnabled` (`/Game/BPs/BP_PickUpItem.StaticMesh` PickUpItem) "QueryAndPhysics")
      (`self.CheckPlacedItem`)
      (return true false))))

(fn `UserConstructionScript`)