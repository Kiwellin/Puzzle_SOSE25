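; A laser puzzle pawn that acts as a beam source or receiver/redirector, which the player rotates in yaw until exiting back to the character.
; Sources trace forward every tick, sizing the Niagara beam to the hit and notifying any laser pawn struck.
; Box hits fire OnHitByLaser and, on redirectors, recursively emit onward.
; A last-hit timestamp limits each pawn to one hit per game time, preventing loops, and switches off unlit beams.
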(event `self.ReceiveBeginPlay`
  (`parent.ReceiveBeginPlay`)
  (`self.SetVFXEnabled` (`self.IsLaserSource`)))

(event `self.ReceiveTick`
  (params (DeltaSeconds :type "Float (single-precision)"))
  ; If source, laser on tick
  (`parent.ReceiveTick` DeltaSeconds)
  (if (`self.IsLaserSource`)
    (`self.EmmitLaser`)
    (elif (`self.TimeHasPassedSinceLastHit`)
      (`self.SetVFXEnabled` false))))

(event `GetHitByLaser`
  (params (HitComponent :type "PrimitiveComponent Object Reference"))
  ; Receive
  (if (== HitComponent (`self.Box`))
    (if (`self.TimeHasPassedSinceLastHit`)
      (set `self.LastHitTime` (`KismetSystemLibrary.GetGameTimeInSeconds`))
      (`self.OnHitByLaser`)
      (if (`self.CanRedirectLight`)
        (`self.SetVFXEnabled` true)
        (`self.EmmitLaser`)))))

(event `EnhancedInput|/Game/Input/Actions/IA_RotateCamera`
  (params (ActionValue :type "Vector2D Structure") (ElapsedSeconds :type "Float (double-precision)") (TriggeredSeconds :type "Float (double-precision)") (InputAction :type "InputAction Object Reference" :default "/Game/Input/Actions/IA_RotateCamera.IA_RotateCamera"))
  ; Controls
  (:`Triggered`
    (`self.K2_AddActorLocalRotation` (`KismetMathLibrary.MakeRotator` 0.0 0.0 (* ActionValue_X (`GameplayStatics.GetWorldDeltaSeconds`) (`self.RotationSpeed`))))))

(event `EnhancedInput|/Game/Input/Actions/IA_ExitPuzzle`
  (params (ActionValue :type Boolean) (ElapsedSeconds :type "Float (double-precision)") (TriggeredSeconds :type "Float (double-precision)") (InputAction :type "InputAction Object Reference" :default "/Game/Input/Actions/IA_ExitPuzzle.IA_ExitPuzzle"))
  ; Controls
  (:`Triggered`
    (`self.Return to Character`)))

(fn `CheckForLaserHit`
  (returns (`Distance to hit` :type "Float (double-precision)") (HitSomething :type Boolean) (`AsBP Laser Pawn` :type "/Game/BPs/LaserPuzzle/BP_LaserPawn Object Reference") (HitComponent :type "PrimitiveComponent Object Reference"))
  (bind _laserorigin (`self.LaserOrigin`))
  (bind _returnvalue (`SceneComponent.K2_GetComponentLocation` _laserorigin))
  (bind (_outhit _returnvalue_2) (`KismetSystemLibrary.LineTraceSingleForObjects` _returnvalue (+ _returnvalue (* (`SceneComponent.GetForwardVector` _laserorigin) (`self.MaxLaserRange`))) (`|MakeArray` "ObjectTypeQuery1" "ObjectTypeQuery2" "ObjectTypeQuery3" "ObjectTypeQuery4" :!type "EObjectTypeQuery Enum")))
  (if _returnvalue_2
    (bind (_bblockinghit _binitialoverlap _time _distance _location _impactpoint _normal _impactnormal _physmat _hitactor _hitcomponent) (`GameplayStatics.BreakHitResult` _outhit))
    (bind _asbp_laser_pawn (cast `/Game/BPs/LaserPuzzle/BP_LaserPawn` _hitactor)
      (:`then`
        _)
      (:`CastFailed`
        _))
    (return (`KismetMathLibrary.VSize` (- _impactpoint (`SceneComponent.K2_GetComponentLocation` (`self.LaserOrigin`)))) _returnvalue_2 _asbp_laser_pawn _hitcomponent)
    (else
      (return 0.0 false null null))))

(fn `EmmitLaser`
  (bind (_distance_to_hit _hitsomething _asbp_laser_pawn _hitcomponent) (`self.CheckForLaserHit`))
  (if _hitsomething
    (`NiagaraComponent.SetVariableFloat` (`self.NS_Laser`) "LaserLength" _distance_to_hit)
    (`/Engine/EditorBlueprintResources/StandardMacros.IsValid` _asbp_laser_pawn
      (:`Is Valid`
        (`self.GetHitByLaser` _asbp_laser_pawn _hitcomponent)))))

(fn `Interact`
  (params (`Player Character` :type "/Game/BPs/BP_FirstPersonCharacter Object Reference") (PickUpItem :type "/Game/BPs/BP_PickUpItem Object Reference"))
  (returns (UsedUpPickUp :type Boolean) (MultiUseItemused :type Boolean))
  (bind _useduppickup (`parent.Interact` `Player Character` PickUpItem))
  (return _useduppickup false))

(fn `SetVFXEnabled`
  (params (IsEnabled :type Boolean))
  (bind _ns_laser (`self.NS_Laser`))
  (if IsEnabled
    (`ActorComponent.Activate` _ns_laser false)
    (else
      (`ActorComponent.Deactivate` _ns_laser))))

(fn `TimeHasPassedSinceLastHit`
  (returns (ReturnValue :type Boolean))
  (return (> (`KismetSystemLibrary.GetGameTimeInSeconds`) (`self.LastHitTime`))))

(fn `UserConstructionScript`
  (`parent.UserConstructionScript`))