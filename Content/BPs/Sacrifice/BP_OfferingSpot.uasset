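; BP_OfferingSpot is a sacrifice spot where an interacted pick-up item is attached and checked against a required item class.
; Interact stores and reparents the item, then runs CheckPlacedItem.
; An offering bowl also needs the correct added ingredient, while other items pass on class alone.
; A correct item notifies the TEST reference to check overall completion, loses its collision and activates a Niagara effect.
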(event `CheckPlacedItem`
  (if (== (`GameplayStatics.GetObjectClass` (`self.PlacedItem`)) (`self.CorrectItem`))
    (bind _returnvalue (`self.CheckIfItemIsOfferingBowl`))
    (if _returnvalue
      (`self.ItemIsCorrect`))))

(event `ItemIsCorrect`
  (`/Game/BPs/Sacrifice/BP_TestAllCorrect.CheckIfAllCorrect` (`self.TEST`))
  (`self.SetActorEnableCollision` (`self.PlacedItem`) false)
  (`ActorComponent.Activate` (`self.Niagara`) false))

(fn `CheckIfItemIsOfferingBowl`
  (returns (ReturnValue :type Boolean))
  (bind _asbp_offering_bowl (cast `/Game/BPs/Sacrifice/BP_OfferingBowl` (`self.PlacedItem`))
    (:`then`
      (bind _addedingredient (`/Game/BPs/Sacrifice/BP_OfferingBowl.AddedIngredient` _asbp_offering_bowl))
      (`/Engine/EditorBlueprintResources/StandardMacros.IsValid` _addedingredient
        (:`Is Valid`
          (if (== (`GameplayStatics.GetObjectClass` _addedingredient) (`self.CorrectIngredient`))
            (return true)))
        (:`Is Not Valid`
          (return false))))
    (:`CastFailed`
      (return true))))

(fn `Interact`
  (params (`Player Character` :type "/Game/BPs/BP_FirstPersonCharacter Object Reference") (PickUpItem :type "/Game/BPs/BP_PickUpItem Object Reference"))
  (returns (UsedUpPickUp :type Boolean))
  (`/Engine/EditorBlueprintResources/StandardMacros.IsValid` PickUpItem
    (:`Is Valid`
      (set `self.PlacedItem` PickUpItem)
      (`/Game/BPs/BP_PickUpItem.ChangeParents` PickUpItem (`self.PlaceBowlHere`))
      (`PrimitiveComponent.SetCollisionEnabled` (`/Game/BPs/BP_PickUpItem.StaticMesh` PickUpItem) "QueryAndPhysics")
      (`self.CheckPlacedItem`)
      (return true))))

(fn `UserConstructionScript`)