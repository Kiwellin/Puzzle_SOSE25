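; BP_OfferingBowl is an interactable bowl in the Sacrifice folder that holds a single ingredient.
; AddIngredient accepts an ingredient only while the bowl has no valid one, then disables its mesh collision, detaches it and snaps it to the ItemHere component, keeping world scale.
; The Interact override calls the parent and always returns false, so placement relies on external calls to AddIngredient.
; A step adding the ingredient to the player's scene capture is left disconnected.
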(event `AddIngredient`
  (params (Ingredient :type "/Game/BPs/Sacrifice/BP_Ingredient Object Reference"))
  (bind _addedingredient (`self.AddedIngredient`))
  (`/Engine/EditorBlueprintResources/StandardMacros.IsValid` _addedingredient
    (:`Is Not Valid`
      (set `self.AddedIngredient` Ingredient)
      (`PrimitiveComponent.SetCollisionEnabled` (`/Game/BPs/Sacrifice/BP_Ingredient.StaticMesh` _addedingredient) "NoCollision")
      (`SceneComponent.K2_DetachFromComponent` (`Actor.RootComponent` Ingredient) "KeepRelative" "KeepRelative" "KeepRelative" true)
      (`self.K2_AttachToComponent` (`self.AddedIngredient`) (`self.ItemHere`) "None" "SnapToTarget" "SnapToTarget" "KeepWorld" true))))

(fn `Interact`
  (params (`Player Character` :type "/Game/BPs/BP_FirstPersonCharacter Object Reference") (PickUpItem :type "/Game/BPs/BP_PickUpItem Object Reference"))
  (returns (UsedUpPickUp :type Boolean))
  (`parent.Interact` `Player Character` PickUpItem)
  (return false))

(fn `UserConstructionScript`
  (`parent.UserConstructionScript`))