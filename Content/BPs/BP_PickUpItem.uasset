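; BP_PickUpItem is a physical item actor that the player character can pick up, carry and drop.
; Interact passes the item to the player character's PickUpItem and returns false.
; ChangeParents turns off physics and collision, then snaps the item onto a given parent component while keeping world scale.
; Drop detaches it in place and restores collision and physics simulation, while DestroySelf removes the actor.
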(event `Drop`
  (`self.K2_DetachFromActor` "KeepWorld" "KeepWorld" "KeepWorld")
  (`PrimitiveComponent.SetCollisionEnabled` (`self.StaticMesh`) "QueryAndPhysics")
  (`PrimitiveComponent.SetSimulatePhysics` (`self.StaticMesh`) true))

(fn `ChangeParents`
  (params (Parent :type "SceneComponent Object Reference"))
  (`PrimitiveComponent.SetSimulatePhysics` (`self.StaticMesh`) false)
  (`PrimitiveComponent.SetCollisionEnabled` (`self.StaticMesh`) "NoCollision")
  (`SceneComponent.K2_DetachFromComponent` (`self.RootComponent`) "KeepRelative" "KeepRelative" "KeepRelative" true)
  (`self.K2_AttachToComponent` Parent "None" "SnapToTarget" "SnapToTarget" "KeepWorld"))

(fn `DestroySelf`
  (`self.K2_DestroyActor`))

(fn `Interact`
  (params (`Player Character` :type "/Game/BPs/BP_FirstPersonCharacter Object Reference") (PickUpItem :type "/Game/BPs/BP_PickUpItem Object Reference"))
  (returns (UsedUpPickUp :type Boolean))
  (`/Game/BPs/BP_FirstPersonCharacter.PickUpItem` `Player Character` self)
  (return false))

(fn `UserConstructionScript`)