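; Spin lock piece that rotates to show the currently selected number, one segment of a spinning lock.
; MoveUpDown steps Number up or down, wraps it around the NumberIndex array, sets TargetRotation from an even division of 360 degrees, and returns the number.
; Tick eases the relative pitch toward that target with a delta-time-scaled, shortest-path rotator lerp.
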(event `self.ReceiveTick`
  (params (DeltaSeconds :type "Float (single-precision)"))
  (`self.K2_SetRelativeRotation` (`KismetMathLibrary.RLerp` (`self.RelativeRotation`) (`KismetMathLibrary.MakeRotator` 0.0 (`self.TargetRotation`) 0.0) (* (`GameplayStatics.GetWorldDeltaSeconds`) 15.0) true)))

(fn `Clamp`
  (`|ExecutionSequence`
    (:`then_0`
      (if (> (`self.Number `) (`KismetArrayLibrary.Array_LastIndex` (`self.NumberIndex`)))
        (set `self.Number ` (- (`self.Number `) (`KismetArrayLibrary.Array_Length` (`self.NumberIndex`))))))
    (:`then_1`
      (if (< (`self.Number `) 0)
        (set `self.Number ` (+ (`self.Number `) (`KismetArrayLibrary.Array_Length` (`self.NumberIndex`))))))))

(fn `MoveUpDown`
  (params (bPickA :type Boolean))
  (returns (Number :type Integer))
  (set `self.Number ` (+ (`self.Number `) (`KismetMathLibrary.SelectInt` 1 -1 bPickA)))
  (`self.Clamp`)
  (set `self.TargetRotation` (* (`KismetMathLibrary.Conv_IntToDouble` (`self.Number `)) (/ 360.0 (`KismetMathLibrary.Conv_IntToDouble` (`KismetArrayLibrary.Array_Length` (`self.NumberIndex`))))))
  (return (`self.Number `)))