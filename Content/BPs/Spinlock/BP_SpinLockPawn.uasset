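; Interactable pawn for a four-piece spinlock combination puzzle that the player operates with directional input.
; Left/right wraps the selection across the pieces, marking it with an overlay highlight.
; Up/down spins the selected piece, and ChangeDisplay rebuilds the text code from each piece's current number.
; A match with CorrectCode after a spin, or the exit input, returns control to the character and clears the highlight.
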(event `self.ReceiveBeginPlay`
  (`parent.ReceiveBeginPlay`)
  (set `self.Pieces` (`|MakeArray` (`self.SpinLockPiece_01`) (`self.SpinLockPiece_02`) (`self.SpinLockPiece_03`) (`self.SpinLockPiece_04`))))

(event `EnhancedInput|/Game/Input/Actions/IA_NavigateRight`
  (params (ActionValue :type Boolean) (ElapsedSeconds :type "Float (double-precision)") (TriggeredSeconds :type "Float (double-precision)") (InputAction :type "InputAction Object Reference" :default "/Game/Input/Actions/IA_NavigateRight.IA_NavigateRight"))
  (:`Triggered`
    (`self.Navigate Pieces` 1)))

(event `EnhancedInput|/Game/Input/Actions/IA_NavigateLeft`
  (params (ActionValue :type Boolean) (ElapsedSeconds :type "Float (double-precision)") (TriggeredSeconds :type "Float (double-precision)") (InputAction :type "InputAction Object Reference" :default "/Game/Input/Actions/IA_NavigateLeft.IA_NavigateLeft"))
  (:`Triggered`
    (`self.Navigate Pieces` -1)))

(event `EnhancedInput|/Game/Input/Actions/IA_ExitPuzzle`
  (params (ActionValue :type Boolean) (ElapsedSeconds :type "Float (double-precision)") (TriggeredSeconds :type "Float (double-precision)") (InputAction :type "InputAction Object Reference" :default "/Game/Input/Actions/IA_ExitPuzzle.IA_ExitPuzzle"))
  (:`Triggered`
    (`self.Return to Character`)))

(event `EnhancedInput|/Game/Input/Actions/IA_NavigateUp`
  (params (ActionValue :type Boolean) (ElapsedSeconds :type "Float (double-precision)") (TriggeredSeconds :type "Float (double-precision)") (InputAction :type "InputAction Object Reference" :default "/Game/Input/Actions/IA_NavigateUp.IA_NavigateUp"))
  (:`Triggered`
    (bind _number (`/Game/BPs/Spinlock/BP_SpinLockPiece.MoveUpDown` (`self.GetSelectedPiece`) true))
    (set `self.CurrentNumberIndexx` _number)
    (`KismetSystemLibrary.PrintString` "up")
    (`self.ChangeDisplay`)
    (if (`self.IsCodeCorrect`)
      (`self.Return to Character`))))

(event `self.Return to Character`
  (`parent.Return to Character`)
  (`self.UpdateHighlightOfSelectedPiece` false))

(event `EnhancedInput|/Game/Input/Actions/IA_NavigateDown`
  (params (ActionValue :type Boolean) (ElapsedSeconds :type "Float (double-precision)") (TriggeredSeconds :type "Float (double-precision)") (InputAction :type "InputAction Object Reference" :default "/Game/Input/Actions/IA_NavigateDown.IA_NavigateDown"))
  (:`Triggered`
    (bind _number (`/Game/BPs/Spinlock/BP_SpinLockPiece.MoveUpDown` (`self.GetSelectedPiece`) false))
    (set `self.CurrentNumberIndexx` _number)
    (`KismetSystemLibrary.PrintString` "down")
    (`self.ChangeDisplay`)
    (if (`self.IsCodeCorrect`)
      (`self.Return to Character`))))

(fn `ChangeDisplay`
  (bind _output (`|GetArrayItem` (`/Game/BPs/Spinlock/BP_SpinLockPiece.Numbers` (`|GetArrayItem` (`self.Pieces`) (`self.CurrentPieceIndex`))) (`self.CurrentNumberIndexx`)))
  (switch `int` (`self.CurrentPieceIndex`)
    (:`0`
      (set `self.A` _output))
    (:`1`
      (set `self.B` _output))
    (:`2`
      (set `self.C` _output))
    (:`3`
      (set `self.D` _output)))
  (`TextRenderComponent.K2_SetText` (`self.CodeDisplay`) (`KismetTextLibrary.Conv_StringToText` (`KismetStringLibrary.Concat_StrStr` (`self.A`) (`self.B`) (`self.C`) (`self.D`))))
  (return))

(fn `GetSelectedPiece`
  (returns (Output :type "/Game/BPs/Spinlock/BP_SpinLockPiece Object Reference"))
  (return (`|GetArrayItem` (`self.Pieces`) (`self.CurrentPieceIndex`))))

(fn `Interact`
  (params (`Player Character` :type "/Game/BPs/BP_FirstPersonCharacter Object Reference") (PickUpItem :type "/Game/BPs/BP_PickUpItem Object Reference"))
  (returns (UsedUpPickUp :type Boolean))
  (bind _useduppickup (`parent.Interact` `Player Character` PickUpItem))
  (`self.UpdateHighlightOfSelectedPiece` true)
  (return _useduppickup))

(fn `IsCodeCorrect`
  (returns (ReturnValue :type Boolean))
  (return (`KismetStringLibrary.EqualEqual_StrStr` (`KismetTextLibrary.Conv_TextToString` (`TextRenderComponent.Text` (`self.CodeDisplay`))) (`self.CorrectCode`))))

(fn `Navigate Pieces`
  (params (Direction :type Integer))
  (`self.UpdateHighlightOfSelectedPiece` false)
  (set `self.CurrentPieceIndex` (+ (`self.CurrentPieceIndex`) Direction))
  (`|ExecutionSequence`
    (:`then_0`
      ;[1 1 1] Make sure index not too high
      (if (> (`self.CurrentPieceIndex`) (`KismetArrayLibrary.Array_LastIndex` (`self.Pieces`)))
        (set `self.CurrentPieceIndex` (- (`self.CurrentPieceIndex`) (`KismetArrayLibrary.Array_Length` (`self.Pieces`))))))
    (:`then_1`
      ;[1 1 1] Make sure index not too low
      (if (< (`self.CurrentPieceIndex`) 0)
        (set `self.CurrentPieceIndex` (+ (`self.CurrentPieceIndex`) (`KismetArrayLibrary.Array_Length` (`self.Pieces`))))))
    (:`then_2`
      ;[1 1 1] Update highlight
      (`self.UpdateHighlightOfSelectedPiece` true))))

(fn `NavigatePiecesUpDown`
  (params (Direction :type Integer))
  (set `self.CurrentNumberIndexx` (+ (`self.CurrentNumberIndexx`) Direction))
  (`|ExecutionSequence`
    (:`then_0`
      (if (> (`self.CurrentNumberIndexx`) (`KismetArrayLibrary.Array_LastIndex` (`/Game/BPs/Spinlock/BP_SpinLockPiece.NumberIndex` (`|GetArrayItem` (`self.Pieces`) (`self.CurrentNumberIndexx`)))))
        (set `self.CurrentNumberIndexx` (- (`self.CurrentNumberIndexx`) (`KismetArrayLibrary.Array_Length` (`/Game/BPs/Spinlock/BP_SpinLockPiece.NumberIndex` (`|GetArrayItem` (`self.Pieces`) (`self.CurrentPieceIndex`))))))))
    (:`then_1`
      (if (< (`self.CurrentNumberIndexx`) 0)
        (set `self.CurrentNumberIndexx` (+ (`self.CurrentNumberIndexx`) (`KismetArrayLibrary.Array_Length` (`/Game/BPs/Spinlock/BP_SpinLockPiece.NumberIndex` (`|GetArrayItem` (`self.Pieces`) (`self.CurrentPieceIndex`))))))))))

(fn `UpdateHighlightOfSelectedPiece`
  (params (bEnabled :type Boolean))
  (`MeshComponent.SetOverlayMaterial` (`self.GetSelectedPiece`) (select `bool` bEnabled :`true` "/Game/Materials/MI_ButtonHighlight.MI_ButtonHighlight" :!type "MaterialInterface Object Reference")))

(fn `UserConstructionScript`
  (`parent.UserConstructionScript`))