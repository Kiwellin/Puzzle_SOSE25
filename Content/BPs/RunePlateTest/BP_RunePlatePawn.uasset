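; Possessable puzzle pawn for a rune plate, where the player traces a code across twelve buttons and returns to the character when it matches.
; Input moves a wrapping highlight in steps of one or three, and interacting lights the rune and spawns a ribbon from the previous one.
; Traces collect labels of crossed buttons into the code compared with CorrectCode.
; Exit or right-click resets materials and code, then fades and destroys ribbons.
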(event `self.ReceiveBeginPlay`
  ;[1 1 1] SETUP
  (set `self.Buttons` (`|MakeArray` (`self.Button_01`) (`self.Button_02`) (`self.Button_03`) (`self.Button_04`) (`self.Button_05`) (`self.Button_06`) (`self.Button_07`) (`self.Button_08`) (`self.Button_09`) (`self.Button_Cancel`) (`self.Button_00`) (`self.Button_Confirm`)))
  (`self.FadeRunes`))

(event `EnhancedInput|/Game/Input/Actions/IA_ExitPuzzle`
  (params (ActionValue :type Boolean) (ElapsedSeconds :type "Float (double-precision)") (TriggeredSeconds :type "Float (double-precision)") (InputAction :type "InputAction Object Reference" :default "/Game/Input/Actions/IA_ExitPuzzle.IA_ExitPuzzle"))
  ;[1 1 1] Possess & Unpossess
  (:`Triggered`
    (`self.Return to Character`)
    (`self.ClearRunes`)))

(event `self.Return to Character`
  ;[1 1 1] Possess & Unpossess
  (`parent.Return to Character`)
  (`self.UpdateHighlightOfSelectedButton` false))

(event `EnhancedInput|/Game/Input/Actions/IA_NavigateRight`
  (params (ActionValue :type Boolean) (ElapsedSeconds :type "Float (double-precision)") (TriggeredSeconds :type "Float (double-precision)") (InputAction :type "InputAction Object Reference" :default "/Game/Input/Actions/IA_NavigateRight.IA_NavigateRight"))
  (:`Triggered`
    (`self.NavigateButtons` 1)))

(event `EnhancedInput|/Game/Input/Actions/IA_NavigateLeft`
  (params (ActionValue :type Boolean) (ElapsedSeconds :type "Float (double-precision)") (TriggeredSeconds :type "Float (double-precision)") (InputAction :type "InputAction Object Reference" :default "/Game/Input/Actions/IA_NavigateLeft.IA_NavigateLeft"))
  (:`Triggered`
    (`self.NavigateButtons` -1)))

(event `EnhancedInput|/Game/Input/Actions/IA_NavigateDown`
  (params (ActionValue :type Boolean) (ElapsedSeconds :type "Float (double-precision)") (TriggeredSeconds :type "Float (double-precision)") (InputAction :type "InputAction Object Reference" :default "/Game/Input/Actions/IA_NavigateDown.IA_NavigateDown"))
  (:`Triggered`
    (`self.NavigateButtons` 3)))

(event `EnhancedInput|/Game/Input/Actions/IA_NavigateUp`
  (params (ActionValue :type Boolean) (ElapsedSeconds :type "Float (double-precision)") (TriggeredSeconds :type "Float (double-precision)") (InputAction :type "InputAction Object Reference" :default "/Game/Input/Actions/IA_NavigateUp.IA_NavigateUp"))
  (:`Triggered`
    (`self.NavigateButtons` -3)))

(event `EnhancedInput|/Game/Input/Actions/IA_Interact`
  (params (ActionValue :type Boolean) (ElapsedSeconds :type "Float (double-precision)") (TriggeredSeconds :type "Float (double-precision)") (InputAction :type "InputAction Object Reference" :default "/Game/Input/Actions/IA_Interact.IA_Interact"))
  (:`Triggered`
    (if (== (`self.GetSelectedButton`) null)
      ;[1 1 1] check if code true
      (if (`self.IsCodeCorrect`)
        (`self.Return to Character`)
        (else
          (`self.FadeRunes`)))
      (else
        ;[1 1 1] Cancel button -> clear display
        (if (not (== (`self.GetSelectedButton`) null))
          ;[1 1 1] Add number to display
          (if (not (`self.IsCodeComplete`))
            (`self.UpdateInteractedButtonLocation`)
            (`PrimitiveComponent.SetMaterial` (`self.GetSelectedButton`) 0 "/Game/Materials/TestRuneHighlight.TestRuneHighlight")
            (`self.DrawLine`)))))))

(event `ClearRunes`
  (set `self.ShowCode` "")
  (`KismetArrayLibrary.Array_Clear` (`self.CurrentCode`))
  (set `self.IsFirstInteract?` true)
  (for _array_element (`self.Buttons`)
    (`PrimitiveComponent.SetMaterial` _array_element 0 "/Engine/EngineMaterials/DefaultMaterial.DefaultMaterial"))
  (`self.FadeRunes`)
  (`KismetSystemLibrary.Delay` 1.0)
  (`self.DestroyRunes`))

(event `Key|RightMouseButton`
  (params (Key :type "Key Structure"))
  (:`Released`
    (`self.ClearRunes`)))

(fn `AddToDisplay`
  (params (`b NumberToAdd` :type String))
  (bind _codedisplay (`self.CodeDisplay`))
  (`TextRenderComponent.K2_SetText` _codedisplay (`KismetTextLibrary.Conv_StringToText` (`KismetStringLibrary.Concat_StrStr` (`KismetTextLibrary.Conv_TextToString` (`TextRenderComponent.Text` _codedisplay)) `b NumberToAdd`))))

(fn `Check if FirstInteract`)

(fn `DestroyRunes`
  (for _array_element (`self.Emitters`)
    (`ActorComponent.K2_DestroyComponent` _array_element))
  (`KismetArrayLibrary.Array_Clear` (`self.Emitters`)))

(fn `DrawLine`
  (bind _interactedbuttonloc (`self.InteractedButtonLoc`))
  (bind _returnvalue (`NiagaraFunctionLibrary.SpawnSystemAtLocation` "/Game/BPs/RunePlateTest/vfx/RuneRibbon.RuneRibbon"))
  (`KismetArrayLibrary.Array_Add` (`self.Emitters`) _returnvalue)
  (if (`self.IsFirstInteract?`)
    (bind _outhits (`KismetSystemLibrary.SphereTraceMultiForObjects` :`Start` _interactedbuttonloc :`End` _interactedbuttonloc :`Radius` 20.0 :`ObjectTypes` (`|MakeArray` "ObjectTypeQuery1" "ObjectTypeQuery2" "ObjectTypeQuery3" :!type "EObjectTypeQuery Enum") :`DrawDebugType` "ForDuration" :`bIgnoreSelf` false))
    (for _array_element _outhits
      (bind _asbp_rune_plate_button (cast `/Game/BPs/RunePlateTest/BP_RunePlateButton` (`.HitComponent` (`GameplayStatics.BreakHitResult` _array_element))))
      (`KismetArrayLibrary.Array_Add` (`self.CurrentCode`) (`/Game/BPs/RunePlateTest/BP_RunePlateButton.ButtonLabel` _asbp_rune_plate_button))
      (set `self.IsFirstInteract?` false))
    (else
      (`FXSystemComponent.SetVectorParameter` _returnvalue "Start pos" (`self.LastInteractedButtonLoc`))
      (`FXSystemComponent.SetVectorParameter` _returnvalue "End pos" (`self.InteractedButtonLoc`))
      (bind _outhits_2 (`KismetSystemLibrary.LineTraceMultiForObjects` :`Start` (`self.LastInteractedButtonLoc`) :`End` (`self.InteractedButtonLoc`) :`ObjectTypes` (`|MakeArray` "ObjectTypeQuery1" "ObjectTypeQuery2" "ObjectTypeQuery3" :!type "EObjectTypeQuery Enum") :`bTraceComplex` true :`DrawDebugType` "ForOneFrame" :`bIgnoreSelf` false))
      (for _array_element_2 _outhits_2
        (bind _asbp_rune_plate_button_2 (cast `/Game/BPs/RunePlateTest/BP_RunePlateButton` (`.HitComponent` (`GameplayStatics.BreakHitResult` _array_element_2))))
        (for _array_element_3 (`|MakeArray` _asbp_rune_plate_button_2)
          (`PrimitiveComponent.SetMaterial` _array_element_3 0 "/Game/Materials/TestRuneHighlight.TestRuneHighlight"))
        (`KismetArrayLibrary.Array_Add` (`self.CurrentCode`) (`/Game/BPs/RunePlateTest/BP_RunePlateButton.ButtonLabel` _asbp_rune_plate_button_2))
        (for _array_element_4 (`self.CurrentCode`)
          (set `self.ShowCode` (`KismetStringLibrary.Concat_StrStr` (`self.ShowCode`) _array_element_4)))
        (if (`self.IsCodeCorrect`)
          (`self.Return to Character`)
          (else
            (`KismetSystemLibrary.PrintString` (`self.ShowCode`))
            (set `self.ShowCode` "")))))))

(fn `FadeRunes`
  (for _array_element (`self.Emitters`)
    (`ActorComponent.Activate` _array_element true)
    (`NiagaraComponent.SetVariableBool` _array_element "Activate" true)))

(fn `GetSelectedButton`
  (returns (Output :type "/Game/BPs/RunePlateTest/BP_RunePlateButton Object Reference"))
  (return (`|GetArrayItem` (`self.Buttons`) (`self.CurrentButtonIndex`))))

(fn `Interact`
  (params (`Player Character` :type "/Game/BPs/BP_FirstPersonCharacter Object Reference") (PickUpItem :type "/Game/BPs/BP_PickUpItem Object Reference"))
  (returns (UsedUpPickUp :type Boolean))
  (`parent.Interact` `Player Character` PickUpItem)
  (`self.UpdateHighlightOfSelectedButton` true)
  (return false))

(fn `IsCodeComplete`
  (returns (ReturnValue :type Boolean))
  (return (== (`KismetStringLibrary.Len` (`KismetTextLibrary.Conv_TextToString` (`TextRenderComponent.Text` (`self.CodeDisplay`)))) (`KismetStringLibrary.Len` (`self.CorrectCode`)))))

(fn `IsCodeCorrect`
  (returns (ReturnValue :type Boolean))
  (return (`KismetStringLibrary.EqualEqual_StrStr` (`self.ShowCode`) (`self.CorrectCode`))))

(fn `NavigateButtons`
  (params (Direction :type Integer))
  (`self.UpdateHighlightOfSelectedButton` false)
  (set `self.CurrentButtonIndex` (+ (`self.CurrentButtonIndex`) Direction))
  (`|ExecutionSequence`
    (:`then_0`
      ;[1 1 1] Make sure index not too high
      (if (> (`self.CurrentButtonIndex`) (`KismetArrayLibrary.Array_LastIndex` (`self.Buttons`)))
        (set `self.CurrentButtonIndex` (- (`self.CurrentButtonIndex`) (`KismetArrayLibrary.Array_Length` (`self.Buttons`))))))
    (:`then_1`
      ;[1 1 1] Make sure index not too low
      (if (< (`self.CurrentButtonIndex`) 0)
        (set `self.CurrentButtonIndex` (+ (`self.CurrentButtonIndex`) (`KismetArrayLibrary.Array_Length` (`self.Buttons`))))))
    (:`then_2`
      ;[1 1 1] Update highlight
      (`self.UpdateHighlightOfSelectedButton` true))))

(fn `UpdateHighlightOfSelectedButton`
  (params (bEnabled :type Boolean))
  (`MeshComponent.SetOverlayMaterial` (`self.GetSelectedButton`) (select `bool` bEnabled :`true` "/Game/Materials/MI_ButtonHighlight.MI_ButtonHighlight" :!type "MaterialInterface Object Reference")))

(fn `UpdateInteractedButtonLocation`
  (if (not (== (`self.InteractedButtonLoc`) (0.0 0.0 0.0)))
    (set `self.LastInteractedButtonLoc` (`self.InteractedButtonLoc`)))
  (set `self.InteractedButtonLoc` (`SceneComponent.K2_GetComponentLocation` (`self.GetSelectedButton`))))

(fn `UserConstructionScript`)