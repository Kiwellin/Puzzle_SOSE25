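; Rune plate socket that turns the correct carried item into a BP_RunePlatePawn when the player interacts with it.
; Interact compares the offered item to CorrectItem, reparents the player's item to PlaceRunePlateHERE, then calls SpawnThePawn.
; SpawnThePawn detaches and destroys the item, then spawns the pawn at that component's transform.
; The RemoveItem and DestroySelf calls are unwired and never run.
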(event `SpawnThePawn`
  (bind _item (`self.Item`))
  (`self.K2_DetachFromActor` _item "KeepRelative" "KeepRelative" "KeepRelative")
  (`self.K2_DestroyActor` _item)
  (`|SpawnActorFromClass` "/Game/BPs/RunePlateTest/BP_RunePlatePawn.BP_RunePlatePawn_C" (`SceneComponent.K2_GetComponentToWorld` (`self.PlaceRunePlateHERE`)) "AlwaysSpawn" "MultiplyWithRoot" null null))

(fn `Interact`
  (params (`Player Character` :type "/Game/BPs/BP_FirstPersonCharacter Object Reference") (PickUpItem :type "/Game/BPs/BP_PickUpItem Object Reference"))
  (returns (UsedUpPickUp :type Boolean))
  (if (== PickUpItem (`self.CorrectItem`))
    (bind _output_get (set `self.Item` (`/Game/BPs/BP_FirstPersonCharacter.Item` `Player Character`)))
    (`/Game/BPs/BP_PickUpItem.ChangeParents` _output_get (`self.PlaceRunePlateHERE`))
    (`self.SpawnThePawn`)
    (return false)))

(fn `UserConstructionScript`)