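; Player controller that routes Enhanced Input to the first-person character.
; On BeginPlay it casts the player pawn to BP_FirstPersonCharacter, caches it and adds the IMP_FirstPersonCharacter mapping context.
; Look input drives yaw and pitch, walk input moves the character along local directions and triggers its walk camera shake on start and completion, and interact calls TryInteract.
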(event `self.ReceiveBeginPlay`
  (bind _asbp_first_person_character (cast `/Game/BPs/BP_FirstPersonCharacter` (`GameplayStatics.GetPlayerCharacter` 0)))
  (set `self.PossessedCharacter` _asbp_first_person_character)
  (`EnhancedInputSubsystemInterface.AddMappingContext` (subsystem `EnhancedInputLocalPlayerSubsystem`) "/Game/Input/IMP_FirstPersonCharacter.IMP_FirstPersonCharacter" 0 (struct)))

(event `EnhancedInput|/Game/Input/IA_RotateCamera`
  (params (ActionValue :type "Vector2D Structure") (ElapsedSeconds :type "Float (double-precision)") (TriggeredSeconds :type "Float (double-precision)") (InputAction :type "InputAction Object Reference" :default "/Game/Input/IA_RotateCamera.IA_RotateCamera"))
  (bind _possessedcharacter (`self.PossessedCharacter`))
  (:`Triggered`
    (`Pawn.AddControllerYawInput` _possessedcharacter ActionValue_X)
    (`Pawn.AddControllerPitchInput` _possessedcharacter ActionValue_Y)))

(event `EnhancedInput|/Game/Input/IA_Walk`
  (params (ActionValue :type "Vector2D Structure") (ElapsedSeconds :type "Float (double-precision)") (TriggeredSeconds :type "Float (double-precision)") (InputAction :type "InputAction Object Reference" :default "/Game/Input/IA_Walk.IA_Walk"))
  (bind _possessedcharacter (`self.PossessedCharacter`))
  (:`Triggered`
    (`/Game/BPs/BP_FirstPersonCharacter.MoveInWorldDirection` _possessedcharacter (`KismetMathLibrary.MakeVector` ActionValue_X ActionValue_Y)))
  (:`Started`
    (`/Game/BPs/BP_FirstPersonCharacter.ShakeCamWalk` _possessedcharacter))
  (:`Completed`
    (`/Game/BPs/BP_FirstPersonCharacter.ShakeCamWalk` _possessedcharacter)))

(event `EnhancedInput|/Game/Input/IA_Interact`
  (params (ActionValue :type Boolean) (ElapsedSeconds :type "Float (double-precision)") (TriggeredSeconds :type "Float (double-precision)") (InputAction :type "InputAction Object Reference" :default "/Game/Input/IA_Interact.IA_Interact"))
  (:`Triggered`
    (`/Game/BPs/BP_FirstPersonCharacter.TryInteract` (`self.PossessedCharacter`))))

(fn `UserConstructionScript`)